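; BP_Jewel_Yellow is a yellow jewel actor in the Volcano area whose point light pulses over time.
; BeginPlay seeds a random phase so separate jewels pulse out of sync.
; Tick advances that phase by delta time and drives the PointLight intensity with an offset degree-based sine, fading smoothly between dark and bright.
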(event `self.ReceiveBeginPlay`
  (set `self.temp` (`KismetMathLibrary.RandomFloatInRange` 0.0 500.0)))

(event `self.ReceiveTick`
  (params (DeltaSeconds :type "Float (single-precision)"))
  (bind _output_get (set `self.temp` (+ (* DeltaSeconds 100.0) (`self.temp`))))
  (`LightComponent.SetIntensity` (`self.PointLight`) (* (+ (`KismetMathLibrary.DegSin` _output_get) 1.0) 40000.0)))

(fn `UserConstructionScript`)