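; BP_FallingStoneZone is a volcano zone actor that continuously spawns BP_FallingStone actors within its Box volume.
; A looping timer started on BeginPlay calls Spawn several times a second, with no limit on count.
; Each stone gets a random rotation, enlarged per-axis scale and offset from the actor's location.
; Offsets use scaled box extents in world axes, covering only the positive half along Y.
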(event `self.ReceiveBeginPlay`
  (`KismetSystemLibrary.K2_SetTimer` null "Spawn" 0.2 true))

(event `Spawn`
  (bind _returnvalue (`KismetMathLibrary.RandomFloatInRange` 2.0 2.5))
  (bind _x (.x (`BoxComponent.GetScaledBoxExtent` (`self.Box`))))
  (bind _y (.y (`BoxComponent.GetScaledBoxExtent` (`self.Box`))))
  (bind _z (.z (`BoxComponent.GetScaledBoxExtent` (`self.Box`))))
  (`|SpawnActorFromClass` "/Game/Volcano/BluePrint/BP_FallingStone.BP_FallingStone_C" (`KismetMathLibrary.MakeTransform` (+ (`KismetMathLibrary.MakeVector` (`KismetMathLibrary.RandomFloatInRange` (* _x -1.0) _x) (`KismetMathLibrary.RandomFloatInRange` (* _y 0.0) _y) (`KismetMathLibrary.RandomFloatInRange` (* _z -1.0) _z)) (`self.K2_GetActorLocation`)) (`KismetMathLibrary.RandomRotator` false) (`KismetMathLibrary.MakeVector` _returnvalue _returnvalue _returnvalue)) "Undefined" "OverrideRootScale" null null))

(fn `UserConstructionScript`)