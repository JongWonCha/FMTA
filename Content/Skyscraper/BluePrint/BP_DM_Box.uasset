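; BP_DM_Box is a breakable box actor that shatters when hit by a bat.
; An overlap between its DestructibleComponent and a BP_BatCollision actor triggers Collapse.
; Collapse applies damage and an impulse at the Arrow component's location along its forward vector, then destroys the actor after a short delay.
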(event `Collapse`
  (bind _arrow (`self.Arrow`))
  (`DestructibleComponent.ApplyDamage` (`self.DestructibleComponent`) 20.0 (`SceneComponent.K2_GetComponentLocation` _arrow) (`SceneComponent.GetForwardVector` _arrow) 20.0)
  (`KismetSystemLibrary.Delay` 2.5)
  (`self.K2_DestroyActor`))

(event `self.DestructibleComponent.OnComponentBeginOverlap`
  (params (OverlappedComponent :type "PrimitiveComponent Object Reference") (OtherActor :type "Actor Object Reference") (OtherComp :type "PrimitiveComponent Object Reference") (OtherBodyIndex :type Integer) (bFromSweep :type Boolean) (SweepResult :type "HitResult Structure (by ref)"))
  (cast `/Game/Characters/Weapon/Bat/BP_BatCollision` OtherActor)
  (if true
    (`self.Collapse`)))

(fn `UserConstructionScript`)