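; BP_LoadingPC is the player controller for a loading screen that bridges travel to the next map.
; On BeginPlay it creates the WidgetBP_Loading widget, adds it to the viewport and waits briefly on a fixed delay.
; It then opens the level named by the NextMap option in the game mode's OptionsString, or only prints a failure if the widget is invalid.
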(event `self.ReceiveBeginPlay`
  (bind _returnvalue (`|CreateWidget` "/Game/UI/Loading/WidgetBP_Loading.WidgetBP_Loading_C" self))
  (bind _output_get (set `self.WidgetBP_Loading` _returnvalue))
  (`/Engine/EditorBlueprintResources/StandardMacros.IsValid` _output_get
    (:`Is Valid`
      (`UserWidget.AddToViewport` _output_get 0)
      (`KismetSystemLibrary.Delay` 1.0)
      (`GameplayStatics.OpenLevel` (`KismetStringLibrary.Conv_StringToName` (`GameplayStatics.ParseOption` (`GameModeBase.OptionsString` (`GameplayStatics.GetGameMode`)) "NextMap"))))
    (:`Is Not Valid`
      (`KismetSystemLibrary.PrintString` "FAIL!"))))

(fn `UserConstructionScript`)