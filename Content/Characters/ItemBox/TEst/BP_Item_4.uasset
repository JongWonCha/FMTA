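; BP_Item_4 is an item pickup that gives a fixed item to Ba_Type or Sp_Type actors on touch.
; Box overlap tries a cast to each type, sets that actor's Item variable to 5, then destroys the pickup.
; Each branch reseeds the Random stream from summed clock fields, but the random integer nodes are unused, so the result never varies.
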(event `self.ReceiveBeginPlay`)

(event `self.Box.OnComponentBeginOverlap`
  (params (OverlappedComponent :type "PrimitiveComponent Object Reference") (OtherActor :type "Actor Object Reference") (OtherComp :type "PrimitiveComponent Object Reference") (OtherBodyIndex :type Integer) (bFromSweep :type Boolean) (SweepResult :type "HitResult Structure (by ref)"))
  (bind (_returnvalue_year _returnvalue_month _returnvalue_day _returnvalue_hour _returnvalue_minute _returnvalue_second _returnvalue_millisecond) (`KismetMathLibrary.BreakDateTime` (`KismetMathLibrary.Now`)))
  (bind (_returnvalue_year_2 _returnvalue_month_2 _returnvalue_day_2 _returnvalue_hour_2 _returnvalue_minute_2 _returnvalue_second_2 _returnvalue_millisecond_2) (`KismetMathLibrary.BreakDateTime` (`KismetMathLibrary.Now`)))
  (`|ExecutionSequence`
    (:`then_0`
      (bind _asba_type (cast `/Game/Characters/Balance/Ba_Type` OtherActor))
      (`KismetMathLibrary.SetRandomStreamSeed` (`self.Random`) (+ _returnvalue_year_2 _returnvalue_month_2 _returnvalue_day_2 _returnvalue_hour_2 _returnvalue_minute_2 _returnvalue_second_2 _returnvalue_millisecond_2))
      (set `/Game/Characters/Balance/Ba_Type.Item` 5 _asba_type)
      (`self.K2_DestroyActor`))
    (:`then_1`
      (bind _assp_type (cast `/Game/Characters/Speed/Sp_Type` OtherActor))
      (`KismetMathLibrary.SetRandomStreamSeed` (`self.Random`) (+ _returnvalue_year _returnvalue_month _returnvalue_day _returnvalue_hour _returnvalue_minute _returnvalue_second _returnvalue_millisecond))
      (set `/Game/Characters/Speed/Sp_Type.Item` 5 _assp_type)
      (`self.K2_DestroyActor`))))

(fn `UserConstructionScript`)