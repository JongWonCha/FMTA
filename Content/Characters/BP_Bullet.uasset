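; Projectile bullet for the battle mode that raises the KnockBack value of Ba, Po and Sp type characters it hits.
; Box overlaps count only on authority while damage is available, skipping the owner's pawn and Ba types with active SkillTime.
; The victim's own ArrowPowerUpTime selects the larger increase.
; A hit hides and stops the bullet, requests impact particles and the owner controller's hit sound, then destroys it.
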(event `self.ReceiveBeginPlay`)

(event `self.ReceiveActorBeginOverlap`
  (params (OtherActor :type "Actor Object Reference")))

(event `self.ReceiveTick`
  (params (DeltaSeconds :type "Float (single-precision)")))

(event `self.Box.OnComponentBeginOverlap`
  (params (OverlappedComponent :type "PrimitiveComponent Object Reference") (OtherActor :type "Actor Object Reference") (OtherComp :type "PrimitiveComponent Object Reference") (OtherBodyIndex :type Integer) (bFromSweep :type Boolean) (SweepResult :type "HitResult Structure (by ref)"))
  (bind _defaultsceneroot (`self.DefaultSceneRoot`))
  (`/Engine/EditorBlueprintResources/ActorMacros.Switch Has Authority`
    (:`Authority`
      (bind _asbp_battle_gs (cast `/Game/Characters/Balance/BP_BattleGS` (`GameplayStatics.GetGameState`)))
      (if (`/Game/Characters/Balance/BP_BattleGS.DamageAvailable` _asbp_battle_gs)
        (`|ExecutionSequence`
          (:`then_0`
            (bind _asba_type (cast `/Game/Characters/Balance/Ba_Type` OtherActor))
            (if (and (<= (`/Game/Characters/Balance/Ba_Type.SkillTime` _asba_type) 0.0001) (!= (`self.GetOwner`) (`Pawn.GetController` _asba_type)))
              (if (> (`/Game/Characters/Balance/Ba_Type.ArrowPowerUpTime` _asba_type) 0.0)
                (bind _knockback (`/Game/Characters/Balance/Ba_Type.KnockBack` _asba_type))
                (set `/Game/Characters/Balance/Ba_Type.KnockBack` (+ _knockback 20.0) _asba_type)
                (else
                  (set `/Game/Characters/Balance/Ba_Type.KnockBack` (+ _knockback 10.0) _asba_type)))
              (`SceneComponent.SetVisibility` (`self.StaticMesh`) false false :!label _label)
              (set `MovementComponent.Velocity` (0.0 0.0 0.0) (`self.ProjectileMovement`))
              (`self.SpawnBulletHitParticle_Req` (+ (`SceneComponent.K2_GetComponentLocation` _defaultsceneroot) (* (`SceneComponent.GetForwardVector` _defaultsceneroot) -100)) (`SceneComponent.K2_GetComponentRotation` _defaultsceneroot))
              (bind _ascharacter_controller (cast `/Game/Characters/Character_Controller` (`self.GetOwner`)))
              (`/Game/Characters/Character_Controller.PlayBulletHitSound_Req` _ascharacter_controller)
              (`self.K2_DestroyActor`)))
          (:`then_1`
            (bind _aspo_type (cast `/Game/Characters/Power/Po_Type` OtherActor))
            (if (!= (`self.GetOwner`) (`Pawn.GetController` _aspo_type))
              (if (> (`/Game/Characters/Power/Po_Type.ArrowPowerUpTime` _aspo_type) 0.0)
                (bind _knockback_2 (`/Game/Characters/Power/Po_Type.KnockBack` _aspo_type))
                (set `/Game/Characters/Power/Po_Type.KnockBack` (+ _knockback_2 20.0) _aspo_type)
                (goto _label)
                (else
                  (set `/Game/Characters/Power/Po_Type.KnockBack` (+ _knockback_2 10.0) _aspo_type)
                  (goto _label)))))
          (:`then_2`
            (bind _assp_type (cast `/Game/Characters/Speed/Sp_Type` OtherActor))
            (if (!= (`self.GetOwner`) (`Pawn.GetController` _assp_type))
              (if (> (`/Game/Characters/Speed/Sp_Type.ArrowPowerUpTime` _assp_type) 0.0)
                (bind _knockback_3 (`/Game/Characters/Speed/Sp_Type.KnockBack` _assp_type))
                (set `/Game/Characters/Speed/Sp_Type.KnockBack` (+ _knockback_3 20.0) _assp_type)
                (goto _label)
                (else
                  (set `/Game/Characters/Speed/Sp_Type.KnockBack` (+ _knockback_3 10.0) _assp_type)
                  (goto _label))))))))))

(event `SpawnBulletHitParticle_Req`
  (params (Location :type "Vector Structure") (Rotation :type "Rotator Structure"))
  (`GameplayStatics.SpawnEmitterAtLocation` "/Game/Characters/Particle/P_BulletHit.P_BulletHit" Location Rotation (1.0 1.0 1.0) true "AutoRelease"))

(fn `UserConstructionScript`)