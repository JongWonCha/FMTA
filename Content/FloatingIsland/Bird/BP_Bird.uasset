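; BP_Bird is a bird actor for the floating island that flies in a straight line and removes itself when out of range.
; Each Tick moves it a fixed step along its Arrow component's forward vector without sweep, so its speed depends on frame rate.
; It then destroys itself once the Arrow's world X or Y leaves a square boundary centered on the world origin.
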(event `self.ReceiveTick`
  (params (DeltaSeconds :type "Float (single-precision)"))
  (bind _arrow (`self.Arrow`))
  (bind (_returnvalue_x _returnvalue_y) (`KismetMathLibrary.BreakVector` (`SceneComponent.K2_GetComponentLocation` (`self.Arrow`))))
  (`|ExecutionSequence`
    (:`then_0`
      (`self.K2_SetActorLocation` (+ (`SceneComponent.K2_GetComponentLocation` _arrow) (* (`KismetMathLibrary.Normal` (`SceneComponent.GetForwardVector` _arrow)) 10.0))))
    (:`then_1`
      (if (or (or (> _returnvalue_x 18000.0) (< _returnvalue_x -18000.0)) (or (> _returnvalue_y 18000.0) (< _returnvalue_y -18000.0)))
        (`self.K2_DestroyActor`)))))

(fn `UserConstructionScript`)