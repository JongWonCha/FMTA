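; BP_Balloon is an air balloon actor for the floating island content that bobs up and down in place.
; BeginPlay randomizes the wave phase and a base height in absolute world Z, so instances move out of step.
; Tick advances the phase with delta time and sets Z to a sine offset around that base, keeping X and Y.
; A height-based destroy check exists but is disconnected.
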(event `self.ReceiveBeginPlay`
  (bind (_returnvalue_x _returnvalue_y) (`KismetMathLibrary.BreakVector` (`SceneComponent.K2_GetComponentLocation` (`self.DefaultSceneRoot`))))
  (bind _returnvalue (`KismetMathLibrary.Conv_IntToDouble` (`KismetMathLibrary.RandomIntegerInRange` -1000 1000)))
  (set `self.Value` (`KismetMathLibrary.Conv_IntToDouble` (`KismetMathLibrary.RandomIntegerInRange` 0 1000)))
  (`self.K2_SetActorLocation` (`KismetMathLibrary.MakeVector` _returnvalue_x _returnvalue_y _returnvalue))
  (set `self.ZLocation` _returnvalue))

(event `self.ReceiveTick`
  (params (DeltaSeconds :type "Float (single-precision)"))
  (bind (_returnvalue_x _returnvalue_y) (`KismetMathLibrary.BreakVector` (`SceneComponent.K2_GetComponentLocation` (`self.DefaultSceneRoot`))))
  (bind _output_get (set `self.Value` (+ (* DeltaSeconds 20.0) (`self.Value`))))
  (`self.K2_SetActorLocation` (`KismetMathLibrary.MakeVector` _returnvalue_x _returnvalue_y (+ (* (`KismetMathLibrary.DegSin` _output_get) 2000.0) (`self.ZLocation`)))))

(fn `UserConstructionScript`)