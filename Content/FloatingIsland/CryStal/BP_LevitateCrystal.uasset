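; BP_LevitateCrystal is a decorative floating crystal actor that continuously bobs up and down while spinning.
; Each Tick moves the Crystal component one unit along Z, using a MoveCount frame counter and the ZMove flag to reverse direction every hundred frames.
; The same Tick adds constant yaw to DefaultSceneRoot.
; Motion ignores delta time, so its speed depends on frame rate.
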(event `self.ReceiveTick`
  (params (DeltaSeconds :type "Float (single-precision)"))
  (bind _defaultsceneroot (`self.DefaultSceneRoot`))
  (`|ExecutionSequence`
    (:`then_0`
      (if (`self.ZMove`)
        (set `self.MoveCount` (+ (`self.MoveCount`) 1))
        (`SceneComponent.K2_SetWorldLocation` (`self.Crystal`) (+ (`SceneComponent.K2_GetComponentLocation` (`self.Crystal`)) (0.0 0.0 1.0)) false false)
        (if (== (`self.MoveCount`) 100)
          (set `self.ZMove` false)
          (set `self.MoveCount` 0))
        (else
          (set `self.MoveCount` (+ (`self.MoveCount`) 1))
          (`SceneComponent.K2_SetWorldLocation` (`self.Crystal`) (+ (`SceneComponent.K2_GetComponentLocation` (`self.Crystal`)) (0.0 0.0 -1.0)) false false)
          (if (== (`self.MoveCount`) 100)
            (set `self.ZMove` true)
            (set `self.MoveCount` 0)))))
    (:`then_1`
      (`SceneComponent.K2_SetWorldRotation` _defaultsceneroot (`KismetMathLibrary.MakeRotator` (.roll (`SceneComponent.K2_GetComponentRotation` _defaultsceneroot)) (.pitch (`SceneComponent.K2_GetComponentRotation` _defaultsceneroot)) (+ (.yaw (`SceneComponent.K2_GetComponentRotation` _defaultsceneroot)) 1.5)) false false))))

(fn `UserConstructionScript`)